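; BP_GridManager builds a level's tile grid from a data table and provides grid lookups.
; The construction script reads tile types and dimensions from the LevelToLoad row of DT_AggLevelData.
; BeginPlay spawns and types a BP_GridTile per cell, storing each in GridTileSet; the BP_Dottie spawn is disconnected.
; Helper functions convert between world, grid and flat-index coordinates and find four-way neighbour indices, using -1 beyond edges.
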(event EventBeginPlay
  (for _index (range 0 (- (* (Variables|Default|GetXLength) (Variables|Default|GetYLength)) 1))
    (bind _returnvalue (Game|SpawnActorfromClass "/Game/TileSystem/BP_GridTile.BP_GridTile_C" (Math|Transform|MakeTransform (Math|Vector|MakeVector (.WorldX (Utilities|GridtoWorld (.GridX (Utilities|IndextoGrid _index)) (.GridY (Utilities|IndextoGrid _index)))) (.WorldY (Utilities|GridtoWorld (.GridX (Utilities|IndextoGrid _index)) (.GridY (Utilities|IndextoGrid _index)))) (Variables|Default|GetZOffset))) "Undefined" 0 0))
    (Default|UpdateType _returnvalue (Utilities|Array|Get(acopy) (Variables|Default|GetTileEnumSet) _index))
    (Utilities|Array|Add (Variables|Default|GetGridTileSet) _returnvalue)))

(fn ConstructionScript
  (bind _returnvalue (Utilities|GetDataTableRow "/Game/TileSystem/LevelSetup/DT_AggLevelData.DT_AggLevelData" (Variables|Default|GetLevelToLoad))
    (:then
      (Variables|Default|SetTileEnumSet (.leveldata _returnvalue))
      (Variables|Default|SetXLength (.xdim _returnvalue))
      (Variables|Default|SetYLength (.ydim _returnvalue)))))

(fn GetAdjacentTiles
  (params (WorldX :type Float%20%28double-precision%29) (WorldY :type Float%20%28double-precision%29))
  (bind (_gridx _gridy) (Utilities|WorldtoGrid WorldX WorldY))
  (LocalVariables|SetGridX _gridx)
  (LocalVariables|SetGridY _gridy)
  ;[1 1 1] Right
  (if (< (LocalVariables|GetGridY) (- (Variables|Default|GetYLength) 1))
    (LocalVariables|Set+Y (Utilities|GridtoIndex (LocalVariables|GetGridX) (+ (LocalVariables|GetGridY) 1)))
    (else
      (LocalVariables|Set+Y -1)))
  ;[1 1 1] Left
  (if (> (LocalVariables|GetGridY) 0)
    (LocalVariables|Set-Y (Utilities|GridtoIndex (LocalVariables|GetGridX) (+ (LocalVariables|GetGridY) -1)))
    (else
      (LocalVariables|Set-Y -1)))
  ;[1 1 1] Top
  (if (< (LocalVariables|GetGridX) (- (Variables|Default|GetXLength) 1))
    (LocalVariables|Set+X (Utilities|GridtoIndex (+ (LocalVariables|GetGridX) 1) (LocalVariables|GetGridY)))
    (else
      (LocalVariables|Set+X -1)))
  ;[1 1 1] Bottom
  (if (> (LocalVariables|GetGridX) 0)
    (LocalVariables|Set-X (Utilities|GridtoIndex (+ (LocalVariables|GetGridX) -1) (LocalVariables|GetGridY)))
    (else
      (LocalVariables|Set-X -1)))
  (return (LocalVariables|Get+X) (LocalVariables|Get-X) (LocalVariables|Get+Y) (LocalVariables|Get-Y)))

(fn GetIndexfromLocation
  (params (Location :type Vector))
  (bind (_gridx _gridy) (Utilities|WorldtoGrid (.x Location) (.y Location)))
  (return (Utilities|GridtoIndex _gridx _gridy)))

(fn GetLocationfromIndex
  (params (Index :type Integer))
  (bind (_gridx _gridy) (Utilities|IndextoGrid Index))
  (bind (_worldx _worldy) (Utilities|GridtoWorld _gridx _gridy))
  (return (Math|Vector|MakeVector _worldx _worldy (Variables|Default|GetZOffset))))