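; Grid tile actor whose type (dirt, stone, hazard, impediment, goal) sets its look and its effect on the player and ladybug.
; UpdateType applies meshes, some randomized from data tables, and materials.
; Player overlap swaps dirt unless Dottie is present; ladybug collision on walkable tiles can trigger win, loss or random impediment.
; A delayed self-calling moss tick grows or decays stone moss, driving material and walkability; hazards face nearby Dottie.
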(event Custom|Event%20MossTick
  (bind _mossgrowing (Variables|Default|GetMossGrowing))
  (Development|PrintString (Utilities|String|BuildString(Integer) "Moss Growing/Level:" (Utilities|String|ToString(Boolean) _mossgrowing) (Variables|Default|GetMossLevel)))
  (if _mossgrowing
    (Utilities|FlowControl|Delay (Variables|Default|GetMossGrowthInterval))
    (else
      (Utilities|FlowControl|Delay (Variables|Default|GetMossDecayInterval))))
  (bind (_mosscap_ _mosszero_) (CallFunction|HandleMossTick))
  (if (and (Variables|Default|GetMossGrowing) _mosscap_)
    (CallFunction|EventStopMossGrowth)
    (CallFunction|EventMossTick)
    (elif (not (and _mosszero_ (not (Variables|Default|GetMossGrowing))))
      (CallFunction|EventMossTick))))

(event Custom|Event%20StartMossGrowth
  (bind _equal (CallFunction|TypeEquals "NewEnumerator2"))
  (if _equal
    (if (Variables|Default|GetMossGrowing)
      _
      (else
        (Variables|Default|SetMossGrowing true)))
    (CallFunction|EventMossTick)))

(event Custom|Event%20StopMossGrowth
  (Variables|Default|SetMossGrowing false))

(event EventBeginPlay)

(event Collision|EventActorBeginOverlap
  (params (OtherActor :type Actor%20Object%20Reference))
  (bind _asbp_third_person_character (Utilities|Casting|CastToBP_ThirdPersonCharacter OtherActor)
    (:then
      (CallFunction|HandlePlayerDirtCollision _asbp_third_person_character))
    (:CastFailed
      (Utilities|Casting|CastToBP_Dottie OtherActor)
      (Variables|Default|SetDottieIsHere true))))

(event EventTick
  (params (DeltaSeconds :type Float%20%28single-precision%29))
  (bind _skeletalaccessory (Variables|Default|GetSkeletalAccessory))
  (bind _returnvalue (Transformation|GetWorldLocation _skeletalaccessory))
  (bind _equal (CallFunction|TypeEquals "NewEnumerator4"))
  (if _equal
    (bind _returnvalue_2 (Actor|GetActorOfClass "/Game/ThirdPerson/Blueprints/BP_Dottie.BP_Dottie_C"))
    (if (<= (Math|Vector|Distance2D(Vector) _returnvalue (Transformation|GetActorLocation _returnvalue_2)) 9e+02)
      (Transformation|SetWorldRotation _skeletalaccessory (Math|Rotator|MakeRotator 0.0 0.0 (+ (.yaw (Math|Rotator|FindLookatRotation _returnvalue (Transformation|GetActorLocation _returnvalue_2))) -9e+01)) false false))))

(event Collision|EventActorEndOverlap
  (params (OtherActor :type Actor%20Object%20Reference))
  (Utilities|Casting|CastToBP_Dottie OtherActor)
  (Variables|Default|SetDottieIsHere false))

(fn ConstructionScript)

(fn UpdateType
  (params (Tile%20Type :type E_TileType%20Enum :default "NewEnumerator0"))
  (bind _skeletalaccessory (Variables|Default|GetSkeletalAccessory))
  (bind _staticaccessory (Variables|Default|GetStaticAccessory))
  (bind _output_get (Variables|Default|SetType Tile%20Type))
  (switch Utilities|FlowControl|Switch|SwitchonE_TileType _output_get
    (:NewEnumerator0
      (bind _returnvalue (Utilities|GetDataTableRow "/Game/TileSystem/Meshes/DT_SkeletalMeshes.DT_SkeletalMeshes" "BasicDirt")
        (:then
          (Class|SkinnedMeshComponent|SetSkeletalMesh _skeletalaccessory (Utilities|Array|Get(acopy) (.mesh _returnvalue) (Math|Random|RandomInteger (Utilities|Array|Length (.mesh _returnvalue)))) true)
          (CallFunction|Random90Rotation _skeletalaccessory)
          (Components|StaticMesh|SetStaticMesh (Variables|Default|GetStaticAccessory) 0))))
    (:NewEnumerator1
      (Class|SkinnedMeshComponent|SetSkeletalMesh (Variables|Default|GetSkeletalAccessory) "/Game/TileSystem/Meshes/Dirt/DirtPath_3.DirtPath_3" true))
    (:NewEnumerator2
      (Utilities|FlowControl|Sequence :!label _label
        (:then_0
          (bind _returnvalue_2 (Utilities|GetDataTableRow "/Game/TileSystem/Meshes/DT_Meshes.DT_Meshes" "Rocks")
            (:then
              (Components|StaticMesh|SetStaticMesh _staticaccessory (Utilities|Array|Get(acopy) (.mesh _returnvalue_2) (Math|Random|RandomInteger (Utilities|Array|Length (.mesh _returnvalue_2))))))))
        (:then_1
          (bind _returnvalue_3 (Rendering|Material|CreateDynamicMaterialInstance _staticaccessory 0 "/Game/TileSystem/Materials/M_BasicStone.M_BasicStone" "None" :!class /Script/Engine.PrimitiveComponent))
          (Variables|Default|SetMaterialInstance _returnvalue_3)
          (CallFunction|UpdateMossMaterial))
        (:then_2
          (CallFunction|Random90Rotation _staticaccessory)
          (Class|SkinnedMeshComponent|SetSkeletalMesh (Variables|Default|GetSkeletalAccessory) "/Game/TileSystem/Meshes/Dirt/DirtPath_3.DirtPath_3" true))))
    (:NewEnumerator3
      (Variables|Default|SetMossLevel (Variables|Default|GetMossCap))
      (goto _label))
    (:NewEnumerator4
      (bind _returnvalue_4 (Utilities|GetDataTableRow "/Game/TileSystem/Meshes/DT_SkeletalMeshes.DT_SkeletalMeshes" "Hazard")
        (:then
          (Class|SkinnedMeshComponent|SetSkeletalMesh (Variables|Default|GetSkeletalAccessory) (Utilities|Array|Get(acopy) (.mesh _returnvalue_4) (Math|Random|RandomInteger (Utilities|Array|Length (.mesh _returnvalue_4)))) true)
          (Rendering|Material|SetMaterial (Variables|Default|GetTileSurface) 0 "/Game/TileSystem/Materials/M_Hazard.M_Hazard"))))
    (:NewEnumerator5
      (Rendering|Material|SetMaterial (Variables|Default|GetTileSurface) 0 "/Game/TileSystem/Materials/M_Impediment.M_Impediment"))
    (:NewEnumerator6
      (Rendering|Material|SetMaterial (Variables|Default|GetTileSurface) 0 "/Game/TileSystem/Materials/M_Goal.M_Goal"))))

(fn GiveDirttoPlayer
  (params (Player :type BP%20Third%20Person%20Character%20Object%20Reference))
  (bind _equal (CallFunction|TypeEquals "NewEnumerator1"))
  (if _equal
    (CallFunction|UpdateType "NewEnumerator0")
    (Default|CollectDirt Player)))

(fn TakeDirtfromPlayer
  (params (Player :type BP%20Third%20Person%20Character%20Object%20Reference))
  (bind _equal (CallFunction|TypeEquals "NewEnumerator0"))
  (if _equal
    (CallFunction|UpdateType "NewEnumerator1")
    (Default|DepositDirt Player)))

(fn HandlePlayerDirtCollision
  (params (Player :type BP%20Third%20Person%20Character%20Object%20Reference))
  (if (not (Variables|Default|GetDottieIsHere))
    (bind _returnvalue (Default|WillDepositDirt Player))
    (if _returnvalue
      (CallFunction|TakeDirtfromPlayer Player)
      (else
        (bind _returnvalue_2 (Default|WillCollectDirt Player))
        (if _returnvalue_2
          (CallFunction|GiveDirttoPlayer Player))))))

(fn TypeEquals
  (params (Type :type E_TileType%20Enum :default "NewEnumerator0"))
  (return (Utilities|Enum|Equal(Enum) (Variables|Default|GetType) Type)))

(fn IsLadybugWalkable
  (bind _equal (CallFunction|TypeEquals "NewEnumerator0"))
  (if _equal
    (return false)
    (else
      (bind _equal_2 (CallFunction|TypeEquals "NewEnumerator2"))
      (if _equal_2
        (return (>= (Variables|Default|GetMossLevel) (Variables|Default|GetWalkableMossThreshold)))
        (else
          (return true))))))

(fn HandleLadybugCollision
  (params (Ladybug :type BP%20Dottie%20Object%20Reference))
  (bind _walkable (CallFunction|IsLadybugWalkable))
  (if _walkable
    (bind _equal (CallFunction|TypeEquals "NewEnumerator4"))
    (if _equal
      (Default|EventGameLost Ladybug)
      (else
        (bind _equal_2 (CallFunction|TypeEquals "NewEnumerator6"))
        (if _equal_2
          (Default|EventGameWon Ladybug)
          (else
            (bind _equal_3 (CallFunction|TypeEquals "NewEnumerator5"))
            (if _equal_3
              (bind _output_get (Variables|Default|SetImpedimentType (Utilities|Enum|ByteToEnumE_ImpedimentType (Math|Conversions|ToByte(Integer) (Math|Random|RandomInteger 3)))))
              (Default|EventImpediment Ladybug _output_get))))))))

(fn HandleMossTick
  (if (Variables|Default|GetMossGrowing)
    ;[1 1 1] GrowMoss
    (bind _result (Math|Integer|IncrementInt (Variables|Default|GetMossLevel))
      (:%20%20
        (if (>= _result (Variables|Default|GetMossCap))
          (Variables|Default|SetMossLevel (Variables|Default|GetMossCap)))
        (LocalVariables|SetMossCapped (>= _result (Variables|Default|GetMossCap)))))
    (else
      ;[1 1 1] LoseMoss
      (bind _result_2 (Math|Integer|DecrementInt (Variables|Default|GetMossLevel))
        (:%20%20
          (if (<= _result_2 0)
            (Variables|Default|SetMossLevel 0))
          (LocalVariables|SetMossZeroed (<= _result_2 0))))))
  (CallFunction|UpdateMossMaterial)
  (return (LocalVariables|GetMossCapped) (LocalVariables|GetMossZeroed)))

(fn UpdateMossMaterial
  (Rendering|Material|SetScalarParameterValue (Variables|Default|GetMaterialInstance) "MossFraction" (/ (Variables|Default|GetMossLevel) (Math|Conversions|ToFloat(Integer) (Variables|Default|GetMossCap))) :!class /Script/Engine.MaterialInstanceDynamic))

(fn Random90Rotation
  (params (Component :type Scene%20Component%20Object%20Reference%20%28by%20ref%29))
  (Transformation|SetRelativeRotation Component (Math|Rotator|MakeRotator 0.0 0.0 (* (Math|Random|RandomInteger 4) 90)) false false))