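; BP_DirtPickup is a collectible dirt pickup that spins in the world until the player rock touches it.
; On overlap with BP_RockPlayer it destroys itself and then calls UpdateDirt on MyGameMode to register the collection.
; Tick applies a local rotation from roll, pitch and yaw speed variables scaled by delta time, so the spin is frame-rate independent.
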(event Collision|EventActorBeginOverlap
  (params (OtherActor :type Actor%20Object%20Reference))
  ;[1 1 1] PickUpCollisionGraph
  (Utilities|Casting|CastToBP_RockPlayer OtherActor)
  (Actor|DestroyActor)
  (bind _asmy_game_mode (Utilities|Casting|CastToMyGameMode (Game|GetGameMode)))
  (Default|UpdateDirt _asmy_game_mode))

(event EventTick
  (params (DeltaSeconds :type Float%20%28single-precision%29))
  ;[1 1 1] RotateCube
  (Transformation|AddActorLocalRotation (* (Math|Rotator|MakeRotator (Variables|Default|GetRollSpeed) (Variables|Default|GetPitchSpeed) (Variables|Default|GetYawSpeed)) DeltaSeconds) false false))

(fn ConstructionScript)