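; MyGameMode is a game mode Blueprint that tracks how much dirt has been collected and shows when the goal is met.
; On BeginPlay it creates the BP_GameUI widget, adds it to the viewport and resets the count.
; UpdateDirt increments the count, pushes it to the widget and calls EndGame, which reveals the all-collected display at five or more.
; An unconnected node for hiding that display never runs.
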(event Custom|ResetGame
  ;[1 1 1] ResetUIGraph
  (Variables|Default|SetcurrentDirtCollected 0)
  (Variables|/Game/RockMovement/BluePrints/BP_GameUI.BP_GameUI_C|SetDirtVar (Variables|Default|GetcurrentUI) 0))

(event Custom|UpdateDirt
  ;[1 1 1] UpdateDirtPointsGraph
  (bind _output_get (Variables|Default|SetcurrentDirtCollected (+ (Variables|Default|GetcurrentDirtCollected) 1)))
  (Variables|/Game/RockMovement/BluePrints/BP_GameUI.BP_GameUI_C|SetDirtVar (Variables|Default|GetcurrentUI) _output_get)
  (CallFunction|EndGame))

(event Custom|EndGame
  ;[1 1 1] EndGameWinGraph
  (if (>= (Variables|Default|GetcurrentDirtCollected) 5)
    (Variables|/Game/RockMovement/BluePrints/BP_GameUI.BP_GameUI_C|SetAllDirtCollectedOpacity (Variables|Default|GetcurrentUI) 1.0)))

(event EventBeginPlay
  ;[1 1 1] AddUIToViewportGraph
  (bind _returnvalue (UserInterface|CreateWidget "/Game/RockMovement/BluePrints/BP_GameUI.BP_GameUI_C"))
  (bind _output_get (Variables|Default|SetcurrentUI _returnvalue))
  (UserInterface|Viewport|AddtoViewport _output_get 0)
  (CallFunction|ResetGame))

(fn ConstructionScript)