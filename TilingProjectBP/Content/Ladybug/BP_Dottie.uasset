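; BP_Dottie is a ladybug that wanders tile to tile across the level's grid on its own.
; RefreshMoveTargets gets the four adjacent tiles from BP_GridManager, keeps the current direction while walkable, and otherwise picks a random valid one.
; Tick updates the target, then refreshes options, when within a small 2D radius of the target.
; While a valid direction exists, it feeds normalized input toward the target into the movement component.
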(event EventBeginPlay
  (CallFunction|RefreshMoveTargets)
  (CallFunction|UpdateTargetLocation))

(event Collision|EventActorBeginOverlap
  (params (OtherActor :type Actor%20Object%20Reference)))

(event EventTick
  (params (DeltaSeconds :type Float%20%28single-precision%29))
  (if (< (Math|Vector|Distance2D(Vector) (Variables|Default|GetTargetLocation) (Transformation|GetActorLocation)) 5e+01)
    (CallFunction|UpdateTargetLocation)
    (CallFunction|RefreshMoveTargets))
  (if (Variables|Default|GetCurrentDirectionValid)
    (CallFunction|MoveLadybug)))

(fn ConstructionScript
  (bind _outactors (Actor|GetAllActorsOfClass "/Game/TileSystem/BP_GridManager.BP_GridManager_C"))
  (Variables|Default|SetGridManager (Utilities|Array|Get(acopy) _outactors)))

(fn UpdateTargetLocation
  (bind _location (Default|GetLocationfromIndex (Variables|Default|GetGridManager) (Utilities|Array|Get(acopy) (Variables|Default|GetMoveOptions) (Variables|Default|GetCurrentDirection))))
  (bind _output_get (Variables|Default|SetTargetLocation _location))
  (return))

(fn UpdateDirection
  (params (Direction :type Integer))
  (Variables|Default|SetCurrentDirection Direction)
  (return))

(fn RefreshMoveTargets
  (bind _returnvalue (Transformation|GetActorLocation))
  (bind _validdirections (LocalVariables|GetValidDirections))
  ;[1 1 1] Refresh MoveOptions
  (bind (_top _bottom _right _left) (Default|GetAdjTiles (Variables|Default|GetGridManager) (.x _returnvalue) (.y _returnvalue)))
  (bind _output_get (Variables|Default|SetMoveOptions (Utilities|Array|MakeArray _top _bottom _right _left)))
  ;[1 1 1] Check if Current Direction is still Valid
  (bind _valid (CallFunction|IsValidMove (Utilities|Array|Get(acopy) _output_get (Variables|Default|GetCurrentDirection))))
  (if _valid
    (CallFunction|UpdateDirection (Variables|Default|GetCurrentDirection))
    (Variables|Default|SetCurrentDirectionValid true)
    (else
      (Utilities|Array|Clear (LocalVariables|GetValidDirections))
      (bind (_array_element _array_index) (Utilities|Array|ForEachLoopwithBreak (Variables|Default|GetMoveOptions))
        (:LoopBody
          (bind _valid_2 (CallFunction|IsValidMove _array_element))
          (if _valid_2
            (Utilities|Array|Add (LocalVariables|GetValidDirections) _array_index)))
        (:Completed
          (bind _output_get_2 (Variables|Default|SetCurrentDirectionValid (Utilities|Array|IsNotEmpty _validdirections)))
          (if _output_get_2
            (CallFunction|UpdateDirection (.OutItem (Utilities|Array|Random _validdirections)))))))))

(fn IsValidMove
  (params (MoveOptionElement :type Integer))
  (bind _gridmanager (Variables|Default|GetGridManager))
  (if (Utilities|Array|IsValidIndex (Variables|/Game/TileSystem/BP_GridManager.BP_GridManager_C|GetGridTileSet _gridmanager) MoveOptionElement)
    (bind _tile (Default|GetTilefromIndex _gridmanager MoveOptionElement))
    (return (and (Utilities|Enum|NotEqual(Enum) (Variables|/Game/TileSystem/BP_GridTile.BP_GridTile_C|GetType _tile) "NewEnumerator0") (Utilities|Enum|NotEqual(Enum) (Variables|/Game/TileSystem/BP_GridTile.BP_GridTile_C|GetType _tile) "NewEnumerator1")))
    (else
      (return false))))

(fn MoveLadybug
  (Class|PawnMovementComponent|AddInputVector (Variables|Default|GetMovementComponent) (Math|Vector|Normalize (- (Variables|Default|GetTargetLocation) (Transformation|GetActorLocation))) false))