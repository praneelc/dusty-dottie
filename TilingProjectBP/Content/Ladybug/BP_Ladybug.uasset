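; Ladybug character that wanders the tile grid, moving from tile to adjacent tile in random directions.
; Construction caches the first BP_GridManager, which supplies the four neighbouring tiles and filters walkability by tile type.
; Each Tick moves a Target component to the destination, picks a random walkable direction when the move is invalid, then applies movement input.
; Arrival requires zero-tolerance location equality; PersistentMoveIsValid is defined but never called.
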(event EventBeginPlay)

(event Collision|EventActorBeginOverlap
  (params (OtherActor :type Actor%20Object%20Reference)))

(event EventTick
  (params (DeltaSeconds :type Float%20%28single-precision%29))
  (Transformation|SetWorldLocation (Variables|Default|GetTarget) (Variables|Default|GetMoveTarget) false true)
  (if (Variables|Default|GetMoveInvalid)
    (CallFunction|GetCardinalMoves)
    (CallFunction|SelectNewDirection))
  (CallFunction|Move))

(fn ConstructionScript
  (bind _outactors (Actor|GetAllActorsOfClass "/Game/TileSystem/BP_GridManager.BP_GridManager_C"))
  (Variables|Default|SetGridManager (Utilities|Array|Get(acopy) _outactors))
  (Variables|Default|SetCurrentDirection (Math|Random|RandomInteger 3))
  (Variables|Default|SetMoveOrigin (Transformation|GetActorLocation)))

(fn GetCardinalMoves
  (bind _returnvalue (Transformation|GetActorLocation))
  (bind (_top _bottom _right _left) (Default|GetAdjTiles (Variables|Default|GetGridManager) (.x _returnvalue) (.y _returnvalue)))
  (for (_array_element _array_index) (Utilities|Array|MakeArray _top _bottom _right _left)
    (Utilities|Array|SetArrayElem (Variables|Default|GetCardinalMoves) _array_index _array_element))
  (for _array_element_2 (Variables|Default|GetCardinalMoves)
    _))

(fn IsWalkableTile
  (params (Tile :type Integer))
  (bind _gridmanager (Variables|Default|GetGridManager))
  (bind _tile (Default|GetTilefromIndex _gridmanager Tile))
  (return (Math|Boolean|ANDBoolean (Utilities|Array|IsValidIndex (Variables|/Game/TileSystem/BP_GridManager.BP_GridManager_C|GetGridTileSet _gridmanager) Tile) (Utilities|Enum|NotEqual(Enum) (Variables|/Game/TileSystem/BP_GridTile.BP_GridTile_C|GetType _tile) "NewEnumerator0") (Utilities|Enum|NotEqual(Enum) (Variables|/Game/TileSystem/BP_GridTile.BP_GridTile_C|GetType _tile) "NewEnumerator1"))))

(fn PersistentMoveIsValid
  (bind _iswalkable (CallFunction|IsWalkableTile (Utilities|Array|Get(acopy) (Variables|Default|GetCardinalMoves) (Variables|Default|GetCurrentDirection))))
  (return _iswalkable))

(fn SelectNewDirection
  (bind _validmoves (LocalVariables|GetValidMoves))
  (Utilities|Array|Clear (LocalVariables|GetValidMoves))
  (for (_array_element _array_index) (Variables|Default|GetCardinalMoves)
    (bind _iswalkable (CallFunction|IsWalkableTile _array_element))
    (if _iswalkable
      (Utilities|Array|Add (LocalVariables|GetValidMoves) _array_index)))
  (if (Utilities|Array|IsNotEmpty _validmoves)
    (Variables|Default|SetCurrentDirection (.OutItem (Utilities|Array|Random _validmoves)))
    (Variables|Default|SetMoveInvalid false)
    (else
      (Variables|Default|SetCurrentDirection -1)
      (Variables|Default|SetMoveInvalid true)))
  (return))

(fn Move
  (bind _location (Default|GetLocationfromIndex (Variables|Default|GetGridManager) (Utilities|Array|Get(acopy) (Variables|Default|GetCardinalMoves) (Variables|Default|GetCurrentDirection))))
  (bind _output_get (Variables|Default|SetMoveTarget _location))
  (if (Utilities|Operators|NotEqual(!=) :A (- _output_get (Transformation|GetActorLocation)))
    (Pawn|Input|AddMovementInput (Class|KismetMathLibrary|VectorNormal2D (- _output_get (Transformation|GetActorLocation)) 0.0001) (Variables|Default|GetMoveSpeed) false)
    (else
      (Variables|Default|SetMoveInvalid true)
      (Variables|Default|SetMoveOrigin (Variables|Default|GetMoveTarget)))))