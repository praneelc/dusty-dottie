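; Grid tile actor with dirt and stone types, each shown by swapping the plane's material.
; Overlap by the third-person character toggles tiles between basic and path dirt, depositing or collecting according to the player's state.
; MakeMossy turns basic stone mossy until a decay delay reverts it.
; GrowMossOnTile runs a delayed MossLevel counter loop while the player spreads moss, without changing the tile type.
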(event Custom|GrowMossOnTile
  (params (Player :type BP%20Third%20Person%20Character%20Object%20Reference))
  (if (Utilities|TileTypeEquals "NewEnumerator1")
    (bind _output_get (Variables|Default|SetReceivingMoss true))
    (Utilities|FlowControl|Delay (Variables|Default|GetMossGrowthTimer))
    ;[1 1 1] SpreadMoss
    (while (and _output_get (Variables|/Game/ThirdPerson/Blueprints/BP_ThirdPersonCharacter.BP_ThirdPersonCharacter_C|GetIsSpreadingMoss Player))
      (bind _result (Math|Integer|IncrementInt (Variables|Default|GetMossLevel))
        (:%20%20
          (if (>= _result (Variables|Default|GetMossCap))
            (Variables|Default|SetReceivingMoss false)
            (else
              (bind _output_get_2 (Variables|Default|SetMossLevel 0))
              (Development|PrintText (Utilities|Text|ToText(Integer) _output_get_2))
              (Utilities|FlowControl|Delay (Variables|Default|GetMossGrowthTimer)))))))
    (Development|PrintString (Utilities|String|ToString(Integer) (Variables|Default|GetMossLevel)))))

(event Custom|Event%20MakeMossy
  (if (Utilities|Enum|Equal(Enum) (Variables|Default|GetType) "NewEnumerator1")
    (CallFunction|SetType "NewEnumerator2")
    (Utilities|FlowControl|Delay (Variables|Default|GetMossDecayTimer))
    (CallFunction|SetType "NewEnumerator1")))

(event EventBeginPlay)

(event Collision|EventActorBeginOverlap
  (params (OtherActor :type Actor%20Object%20Reference))
  (bind _asbp_third_person_character (Utilities|Casting|CastToBP_ThirdPersonCharacter OtherActor))
  (if (Variables|/Game/ThirdPerson/Blueprints/BP_ThirdPersonCharacter.BP_ThirdPersonCharacter_C|GetDirtDepositing _asbp_third_person_character)
    (bind _candeposit (Default|CanDepositDirt _asbp_third_person_character))
    (if _candeposit
      (CallFunction|DepositDirt _asbp_third_person_character))
    (else
      (bind _can_collect (Default|CanCollectDirt _asbp_third_person_character))
      (if _can_collect
        (CallFunction|TakeDirt _asbp_third_person_character)))))

(fn ConstructionScript)

(fn Instantiate
  (params (Type :type E_TileTypes%20Enum :default "NewEnumerator0"))
  (CallFunction|SetType Type))

(fn SetType
  (params (Type :type E_TileTypes%20Enum :default "NewEnumerator0"))
  (bind _plane (Variables|Default|GetPlane))
  (Development|PrintString (Utilities|String|Append (Utilities|String|MakeLiteralString "Tile was") (Utilities|String|EnumtoString Type)))
  (bind _output_get (Variables|Default|SetType Type))
  (Development|PrintString (Utilities|String|Append (Utilities|String|MakeLiteralString "Tile is now") (Utilities|String|EnumtoString _output_get)))
  (switch Utilities|FlowControl|Switch|SwitchonE_TileTypes Type
    (:NewEnumerator0
      (Rendering|Material|SetMaterial _plane 0 "/Game/TileSystem/TileMaterials/M_BasicDirt.M_BasicDirt"))
    (:NewEnumerator4
      (Rendering|Material|SetMaterial _plane 0 "/Game/TileSystem/TileMaterials/M_PathDirt.M_PathDirt"))
    (:NewEnumerator1
      (Rendering|Material|SetMaterial _plane 0 "/Game/TileSystem/TileMaterials/M_BasicStone.M_BasicStone"))
    (:NewEnumerator2
      (Rendering|Material|SetMaterial (Variables|Default|GetPlane) 0 "/Game/TileSystem/TileMaterials/M_MossyStone.M_MossyStone"))))

(fn TakeDirt
  (params (Player :type BP%20Third%20Person%20Character%20Object%20Reference))
  (if (Utilities|TileTypeEquals "NewEnumerator4")
    (CallFunction|SetType "NewEnumerator0")
    (Default|CollectDirt Player)))

(fn DepositDirt
  (params (Player :type BP%20Third%20Person%20Character%20Object%20Reference))
  (if (Utilities|TileTypeEquals "NewEnumerator0")
    (CallFunction|SetType "NewEnumerator4")
    (Default|DepositDirt Player)))