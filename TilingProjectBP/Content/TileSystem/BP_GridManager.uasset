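; Grid manager that builds a Width-by-Height board of randomly typed BP_GridTile actors.
; The Construction Script fills TileEnumSet with random tile types, and BeginPlay spawns a tile per index, instantiates it with its type and stores it in GridTileSet.
; GetAdjTiles converts a world position to a grid index and returns the four orthogonal neighbor indices, using -1 beyond the edges.
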(event EventBeginPlay
  (for _index (range 0 (- (* (Variables|Default|GetWidth) (Variables|Default|GetHeight)) 1))
    (bind _returnvalue (Game|SpawnActorfromClass "/Game/TileSystem/BP_GridTile.BP_GridTile_C" (Math|Transform|MakeTransform (Math|Vector|MakeVector (Math|Conversions|ToFloat(Integer) (.Width (Utilities|IndextoGrid _index))) (Math|Conversions|ToFloat(Integer) (.Height (Utilities|IndextoGrid _index))) 2.0)) "Undefined" 0 0))
    (Default|Instantiate _returnvalue (Utilities|Array|Get(acopy) (Variables|Default|GetTileEnumSet) _index))
    (Utilities|Array|Add (Variables|Default|GetGridTileSet) _returnvalue)))

(event Collision|EventActorBeginOverlap
  (params (OtherActor :type Actor%20Object%20Reference)))

(event EventTick
  (params (DeltaSeconds :type Float%20%28single-precision%29)))

(fn ConstructionScript
  (for _index (range 0 (- (* (Variables|Default|GetWidth) (Variables|Default|GetHeight)) 1))
    (Utilities|Array|SetArrayElem (Variables|Default|GetTileEnumSet) _index (Utilities|Enum|ByteToEnumE_TileTypes (Math|Conversions|ToByte(Integer) (Math|Random|RandomInteger 5))) true)))

(fn GetAdjTiles
  (params (X :type Float%20%28double-precision%29) (Y :type Float%20%28double-precision%29))
  (bind (_gridw _gridh) (Utilities|WorldtoGrid X Y))
  (LocalVariables|SetGridX _gridw)
  (LocalVariables|SetGridY _gridh)
  (LocalVariables|SetIndex (Utilities|GridtoIndex _gridw _gridh))
  (Utilities|FlowControl|Sequence
    (:then_0
      ;[1 1 1] Get Top Cell
      (if (< (LocalVariables|GetGridY) (- (Variables|Default|GetHeight) 1))
        (LocalVariables|SetOutTop (+ (LocalVariables|GetIndex) (Variables|Default|GetWidth)))
        (else
          (LocalVariables|SetOutTop -1)))
      ;[1 1 1] Get Bottom Cell
      (if (> (LocalVariables|GetGridY) 0)
        (LocalVariables|SetOutBot (- (LocalVariables|GetIndex) (Variables|Default|GetWidth)))
        (else
          (LocalVariables|SetOutBot -1)))
      ;[1 1 1] Get Right Cell
      (if (< (LocalVariables|GetGridX) (- (Variables|Default|GetWidth) 1))
        (LocalVariables|SetOutRight (+ (LocalVariables|GetIndex) 1))
        (else
          (LocalVariables|SetOutRight -1)))
      ;[1 1 1] Get Left Cell
      (if (> (LocalVariables|GetGridX) 0)
        (LocalVariables|SetOutLeft (- (LocalVariables|GetIndex) 1))
        (else
          (LocalVariables|SetOutLeft -1)))
      ;[1 1 1] Outputs
      (return (LocalVariables|GetOutTop) (LocalVariables|GetOutBot) (LocalVariables|GetOutRight) (LocalVariables|GetOutLeft)))))